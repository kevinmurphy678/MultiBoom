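; Interactable light switch that toggles its Light component when the player presses Interact while overlapping its Trigger, which enables and disables input.
; SetLight applies visibility, plays a press sound pitched lower when off, and runs a guarded timeline that nudges the button mesh; BeginPlay also calls it.
; ToggleLight additionally calls PerformAction on an optional Performer.
; The construction script sets default visibility and tints the light and a dynamic mesh material with Color.
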(event OnComponentBeginOverlap(Trigger)
  (params (OverlappedComponent :type Primitive%20Component%20Object%20Reference) (OtherActor :type Actor%20Object%20Reference) (OtherComp :type Primitive%20Component%20Object%20Reference) (OtherBodyIndex :type Integer) (bFromSweep :type Boolean) (SweepResult :type Hit%20Result%20Structure%20%28by%20ref%29))
  (Input|EnableInput (Game|GetPlayerController 0)))

(event OnComponentEndOverlap(Trigger)
  (params (OverlappedComponent :type Primitive%20Component%20Object%20Reference) (OtherActor :type Actor%20Object%20Reference) (OtherComp :type Primitive%20Component%20Object%20Reference) (OtherBodyIndex :type Integer))
  (Input|DisableInput (Game|GetPlayerController 0)))

(event Custom|Set%20Light
  (params (Visbility :type Boolean))
  (bind _press (Variables|Default|GetPress))
  (bind _pitch (Variables|Default|GetPitch))
  (bind _light (Variables|Default|GetLight))
  ;[1 1 1] Toggle Light
  (Rendering|SetVisibility _light Visbility false)
  (if (Rendering|IsVisible _light)
    (Variables|Default|Setvisibility true)
    (Variables|/Script/Engine.AudioComponent|SetPitchMultiplier _press _pitch)
    (else
      (Variables|Default|Setvisibility false)
      (Variables|/Script/Engine.AudioComponent|SetPitchMultiplier _press (* 0.75 _pitch))))
  (Audio|Components|Audio|Play _press 0.0)
  (if (not (Variables|Default|Getanimating))
    (Variables|Default|Setanimating true)
    (bind _press_2 (Timeline|Button_Press PlayFromStart)
      (:Update
        (Transformation|AddRelativeLocation (Variables|Default|GetStaticMesh2) (Math|Vector|MakeVector 0.0 _press_2 0.0) false false))
      (:Finished
        (Variables|Default|Setanimating false)))))

(event Custom|ToggleLight
  (params (visible :type Boolean))
  (bind _performer (Variables|Default|GetPerformer))
  ;[1 1 1] Toggle Light
  (CallFunction|SetLight visible)
  (Utilities|IsValid (Utilities|ToObject(Interface) _performer)
    (:Is%20Valid
      (Default|PerformAction _performer))))

(event EventBeginPlay
  ;[1 1 1] Toggle Light
  (if (Variables|Default|Getvisibility)
    (CallFunction|SetLight true)
    (else
      (CallFunction|SetLight false))))

(event EventInteract
  ;[1 1 1] Toggle Light
  (CallFunction|ToggleLight (not (Rendering|IsVisible (Variables|Default|GetLight)))))

(fn ConstructionScript
  (bind _light (Variables|Default|GetLight))
  (bind _color (Variables|Lighting|GetColor))
  (Rendering|SetVisibility _light (Variables|Lighting|GetDefault%20Visibility) false)
  (Rendering|Components|Light|SetLightColor _light _color true)
  (bind _returnvalue (Rendering|Material|CreateDynamicMaterialInstance "/Game/Materials/M_Basic_Wall.M_Basic_Wall" :!class /Script/Engine.KismetMaterialLibrary))
  (bind _output_get (Variables|Default|Setmat _returnvalue))
  (Rendering|Material|SetVectorParameterValue _output_get "Color" _color :!class /Script/Engine.MaterialInstanceDynamic)
  (Rendering|Material|SetMaterial (Variables|Default|GetStaticMesh) 0 (Variables|Default|Getmat)))