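; An actor Blueprint that shows web pages through a WebBrowser inside its "lol" user widget.
; On BeginPlay it waits briefly, then loads the idle URL.
; PerformAction toggles between the main URL and the idle URL, tracking the current state with IsPlaying.
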(event EventBeginPlay
  (Utilities|FlowControl|Delay 1.0)
  (bind _aslol (Utilities|Casting|CastTolol (UserInterface|GetUserWidgetObject (Variables|Default|GetWidget))))
  (Class|WebBrowser|LoadURL (Variables|/Game/Blueprints/misc/lol.lol_C|GetWebBrowser_38 _aslol) (Variables|Default|GetIDLE_URL)))

(event EventPerformAction
  (bind _aslol (Utilities|Casting|CastTolol (UserInterface|GetUserWidgetObject (Variables|Default|GetWidget))))
  (if (Variables|Default|GetIsPlaying)
    (Class|WebBrowser|LoadURL (Variables|/Game/Blueprints/misc/lol.lol_C|GetWebBrowser_38 _aslol) (Variables|Default|GetIDLE_URL))
    (Variables|Default|SetIsPlaying false)
    (else
      (Class|WebBrowser|LoadURL (Variables|/Game/Blueprints/misc/lol.lol_C|GetWebBrowser_38 _aslol) (Variables|Default|GetURL))
      (Variables|Default|SetIsPlaying true))))

(fn ConstructionScript)