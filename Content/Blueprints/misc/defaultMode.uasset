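; Game mode Blueprint that handles player respawning.
; On BeginPlay it caches all PlayerStart actors, and Respawn spawns a MemePlayerCharacter with preset health at a random one, using only that start's location.
; The given controller possesses the new character, then, if it is a MemePlayerController, refreshes its client HUD.
; A separate GetAllPlayers event stores every MemePlayerController in a Players list.
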(event Custom|Respawn
  (params (controller :type Player%20Controller%20Object%20Reference))
  (bind _spawns (Variables|Default|Getspawns))
  (Development|PrintString "Spawn requested..")
  (Utilities|IsValid controller
    (:Is%20Valid
      (bind _returnvalue (Game|SpawnActorfromClass "/Game/Blueprints/player/memePlayerCharacter.MemePlayerCharacter_C" (Math|Conversions|ToTransform(Vector) (Transformation|GetActorLocation (Utilities|Array|Get(acopy) _spawns (Math|Random|RandomIntegerinRange 0 (Utilities|Array|LastIndex _spawns))))) "Undefined" controller 500 500))
      (Pawn|Possess controller _returnvalue)
      (Development|PrintString "spawning...")
      (bind _asmeme_player_controller (Utilities|Casting|CastToMemePlayerController controller))
      (Default|UPDATEHUDonCLIENT _asmeme_player_controller _returnvalue))))

(event Custom|GetAllPlayers
  (bind _outactors (Actor|GetAllActorsOfClass "/Game/Blueprints/player/MemePlayerController.MemePlayerController_C"))
  (Variables|Default|Setplayers _outactors))

(event EventBeginPlay
  (bind _outactors (Actor|GetAllActorsOfClass "/Script/Engine.PlayerStart"))
  (Variables|Default|Setspawns _outactors))

(event EventTick
  (params (DeltaSeconds :type Float%20%28single-precision%29)))

(fn ConstructionScript)