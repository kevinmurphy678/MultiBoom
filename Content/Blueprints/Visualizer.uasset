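; Music visualizer actor that plays a song loaded from disk and drives height changes on cube actors by frequency band.
; On BeginPlay the SoundVis component loads the file under the game root and feeds the wave into the Audio component's sound parameter.
; Play and Stop toggle playback and spectrum calculation together.
; Each spectrum update averages seven bands, sub-bass to brilliance, and calls AdjustHeight on that band's cube class with per-band scaling.
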(event OnFrequencySpectrumCalculated(SoundVis)
  (params (OutFrequencies :type Array%20of%20Floats%20%28single-precision%29))
  (Variables|Default|Setfreqs OutFrequencies)
  (Utilities|FlowControl|Sequence
    (:then_0
      (bind _outactors (Actor|GetAllActorsOfClass "/Game/Blueprints/SoundTestBPs/Blueprints/Cubes/SubBassCube.SubBassCube_C"))
      (Default|AdjustHeight _outactors (Class|SoundVisComponent|GetAverageFrequencyValueinRange (Variables|Default|Getsound_wave) (Variables|Default|Getfreqs) 20 60) 9e+05))
    (:then_1
      (bind _outactors_2 (Actor|GetAllActorsOfClass "/Game/Blueprints/SoundTestBPs/Blueprints/Cubes/BassCube.BassCube_C"))
      (Default|AdjustHeight _outactors_2 (Class|SoundVisComponent|GetAverageFrequencyValueinRange (Variables|Default|Getsound_wave) (Variables|Default|Getfreqs) 60 250) 5e+05))
    (:then_2
      (bind _outactors_3 (Actor|GetAllActorsOfClass "/Game/Blueprints/SoundTestBPs/Blueprints/Cubes/LowMidCube.LowMidCube_C"))
      (Default|AdjustHeight _outactors_3 (Class|SoundVisComponent|GetAverageFrequencyValueinRange (Variables|Default|Getsound_wave) (Variables|Default|Getfreqs) 250 500) 2e+05))
    (:then_3
      (bind _outactors_4 (Actor|GetAllActorsOfClass "/Game/Blueprints/SoundTestBPs/Blueprints/Cubes/MidCub.MidCub_C"))
      (Default|AdjustHeight _outactors_4 (Class|SoundVisComponent|GetAverageFrequencyValueinRange (Variables|Default|Getsound_wave) (Variables|Default|Getfreqs) 500 2000) 8e+04))
    (:then_4
      (bind _outactors_5 (Actor|GetAllActorsOfClass "/Game/Blueprints/SoundTestBPs/Blueprints/Cubes/HighMidCube.HighMidCube_C"))
      (Default|AdjustHeight _outactors_5 (Class|SoundVisComponent|GetAverageFrequencyValueinRange (Variables|Default|Getsound_wave) (Variables|Default|Getfreqs) 2000 4000) 5e+04))
    (:then_5
      (bind _outactors_6 (Actor|GetAllActorsOfClass "/Game/Blueprints/SoundTestBPs/Blueprints/Cubes/PresenceCube.PresenceCube_C"))
      (Default|AdjustHeight _outactors_6 (Class|SoundVisComponent|GetAverageFrequencyValueinRange (Variables|Default|Getsound_wave) (Variables|Default|Getfreqs) 4000 6000) 3.5e+04))
    (:then_6
      (bind _outactors_7 (Actor|GetAllActorsOfClass "/Game/Blueprints/SoundTestBPs/Blueprints/Cubes/BrillianceCube.BrillianceCube_C"))
      (Default|AdjustHeight _outactors_7 (Class|SoundVisComponent|GetAverageFrequencyValueinRange (Variables|Default|Getsound_wave) (Variables|Default|Getfreqs) 6000 16000) 1.5e+04))))

(event OnFileLoadCompleted(SoundVis)
  (params (SoundWaveRef :type Sound%20Wave%20Object%20Reference))
  (bind _output_get (Variables|Default|Setsound_wave SoundWaveRef))
  (Class|AudioComponent|SetWaveParameter (Variables|Default|GetAudio) "sound1" _output_get))

(event Custom|Play
  (Audio|Components|Audio|Play (Variables|Default|GetAudio) 0.0)
  (Class|SoundVisComponent|StartCalculatingFrequencySpectrum (Variables|Default|GetSoundVis) (stale OnFileLoadCompleted(SoundVis) _output_get) 0.1))

(event Custom|Stop
  (Audio|Components|Audio|Stop (Variables|Default|GetAudio))
  (Class|SoundVisComponent|StopCalculatingFrequencySpectrum (Variables|Default|GetSoundVis)))

(event EventBeginPlay
  (bind _returnvalue (Class|VictoryBPFunctionLibrary|VictoryPathsGameRootDirectory))
  (bind _song_ (Variables|Default|GetSong%20))
  (bind _returnvalue_2 (Utilities|String|Append _returnvalue _song_))
  (Class|SoundVisComponent|LoadSoundFilefromHD (Variables|Default|GetSoundVis) _returnvalue_2)
  (Development|PrintString _returnvalue_2 true true "(R=0.000000,G=0.660000,B=1.000000,A=1.000000)" 6.0))

(event Collision|EventActorBeginOverlap
  (params (OtherActor :type Actor%20Object%20Reference)))

(fn ConstructionScript)

(fn OnRepSong)