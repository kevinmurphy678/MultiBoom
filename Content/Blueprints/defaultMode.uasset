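; defaultMode is a game mode-style Blueprint that respawns a controller as a new ThirdPersonCharacter.
; BeginPlay caches every PlayerStart actor in Spawns.
; The Respawn event checks the controller, spawns the character at the first cached start's location and possesses it, printing debug messages.
; A random-index node is left unconnected, so spawn selection is not randomized.
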(event Custom|Respawn
  (params (controller :type Player%20Controller%20Object%20Reference))
  (Development|PrintString "Spawn requested..")
  (Utilities|IsValid controller
    (:Is%20Valid
      (bind _returnvalue (Game|SpawnActorfromClass "/Game/Blueprints/ThirdPersonCharacter.ThirdPersonCharacter_C" (Math|Conversions|ToTransform(Vector) (Transformation|GetActorLocation (Utilities|Array|Get(acopy) (Variables|Default|Getspawns)))) "Undefined" 0 0))
      (Pawn|Possess controller _returnvalue)
      (Development|PrintString "spawning..."))))

(event EventBeginPlay
  (bind _outactors (Actor|GetAllActorsOfClass "/Script/Engine.PlayerStart"))
  (Variables|Default|Setspawns _outactors))

(event EventTick
  (params (DeltaSeconds :type Float%20%28single-precision%29)))

(fn ConstructionScript)