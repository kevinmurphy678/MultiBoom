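; A server-authoritative physics object that carries a configurable mesh and damages player characters it hits.
; The authority records the mesh transform each tick, while remote instances, which also simulate physics, interpolate their mesh toward that stored transform.
; On the authority, hits on a MemePlayerCharacter apply physics damage scaled by mass and velocity, with a speed check that always passes.
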(event EventBeginPlay
  (Networking|SwitchHasAuthority
    (:Remote
      (Variables|Default|SetwtClient (Transformation|GetWorldTransform (Variables|Default|GetSM))))))

(event Collision|EventActorBeginOverlap
  (params (OtherActor :type Actor%20Object%20Reference)))

(event EventTick
  (params (DeltaSeconds :type Float%20%28single-precision%29))
  (bind _sm (Variables|Default|GetSM))
  (Networking|SwitchHasAuthority
    (:Authority
      (Variables|Default|SetworldTransform (Transformation|GetWorldTransform (Variables|Default|GetSM))))
    (:Remote
      (Variables|Default|SetwtClient (Transformation|GetWorldTransform _sm))
      (Transformation|SetWorldTransform _sm (Class|KismetMathLibrary|TInterpto (Variables|Default|GetwtClient) (Variables|Default|GetworldTransform) DeltaSeconds 3.0) false false))))

(event Collision|EventHit
  (params (MyComp :type Primitive%20Component%20Object%20Reference) (Other :type Actor%20Object%20Reference) (OtherComp :type Primitive%20Component%20Object%20Reference) (bSelfMoved :type Boolean) (HitLocation :type Vector :default "0, 0, 0") (HitNormal :type Vector :default "0, 0, 0") (NormalImpulse :type Vector :default "0, 0, 0") (Hit :type Hit%20Result%20Structure%20%28by%20ref%29))
  (bind _self self)
  (bind _returnvalue (Transformation|GetVelocity _self))
  (bind _returnvalue_2 (Math|Vector|VectorLength _returnvalue))
  (Networking|SwitchHasAuthority
    (:Authority
      (bind _asmeme_player_character (Utilities|Casting|CastToMemePlayerCharacter Other))
      (if (>= _returnvalue_2 0.0)
        (Game|Damage|ApplyDamage _asmeme_player_character (* (Physics|GetMass (Variables|server_physicsobject_C|GetSM _self)) (/ _returnvalue_2 3e+03)) 0 _self "/Game/Data/DT_Physics.DT_Physics_C")))))

(fn ConstructionScript
  (bind _sm (Variables|Default|GetSM))
  (bind _mesh (Variables|Default|GetMesh))
  (bind _sm_2 (Variables|Default|GetSM))
  (Networking|SwitchHasAuthority
    (:Authority
      (Physics|SetSimulatePhysics _sm_2 true)
      (Variables|Default|SetworldTransform (Transformation|GetWorldTransform _sm_2))
      (Components|StaticMesh|SetStaticMesh _sm_2 _mesh))
    (:Remote
      (Physics|SetSimulatePhysics _sm_2 true)
      (Variables|Default|SetwtClient (Transformation|GetWorldTransform _sm))
      (Components|StaticMesh|SetStaticMesh _sm _mesh))))