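; Meme-themed sticky grenade item that latches onto the first physics-simulating object it hits, then explodes.
; On that hit, a DoOnce attaches the mesh to the other actor's root and starts a timed chain: beeping, meme sound, force impulse, explosion effect and sound, then self-destruction.
; Hits on non-physics surfaces play a boing, filtered by distance from the last boing location to limit repeats.
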(event EventBeginPlay)

(event Collision|EventActorBeginOverlap
  (params (OtherActor :type Actor%20Object%20Reference)))

(event EventTick
  (params (DeltaSeconds :type Float%20%28single-precision%29)))

(event Collision|EventHit
  (params (MyComp :type Primitive%20Component%20Object%20Reference) (Other :type Actor%20Object%20Reference) (OtherComp :type Primitive%20Component%20Object%20Reference) (bSelfMoved :type Boolean) (HitLocation :type Vector) (HitNormal :type Vector) (NormalImpulse :type Vector :default "0, 0, 0") (Hit :type Hit%20Result%20Structure%20%28by%20ref%29))
  (bind _returnvalue (Physics|IsSimulatingPhysics OtherComp "None"))
  (bind _staticmesh (Variables|Default|GetStaticMesh))
  (bind _returnvalue_2 (Transformation|GetWorldLocation _staticmesh))
  (Utilities|FlowControl|Sequence
    (:then_0
      (if _returnvalue
        (Utilities|FlowControl|DoOnce false
          (:Completed
            (Class|SceneComponent|Attachto (Variables|Default|GetStaticMesh) (VehicleSound|GetRootComponent Other) "None" "KeepWorldPosition" true)
            (Audio|SpawnSoundAttached "/Game/Sound/beepbeep.beepbeep" (Variables|Default|GetStaticMesh) "None" "0, 0, 0" "0, 0, 0" "SnapToTarget")
            (Utilities|FlowControl|Delay 5.0)
            (Audio|PlaySoundatLocation "/Game/Sound/idubbbz_burpspotted.idubbbz_burpspotted" _returnvalue_2)
            (Utilities|FlowControl|Delay 1.8)
            (Class|RadialForceComponent|FireImpulse (Variables|Default|GetExplodeyForcey))
            (Utilities|FlowControl|Delay 0.02)
            (Effects|SpawnEmitteratLocation "/Game/Particles/P_Explosion.P_Explosion" _returnvalue_2)
            (Audio|PlaySoundatLocation "/Game/Sound/splode.splode" _returnvalue_2 "0, 0, 0" 4.0)
            (Actor|DestroyActor)))))
    (:then_1
      (if (and (>= (Math|Vector|VectorLength (- (stale _output_get) HitLocation)) 3.0) (not _returnvalue))
        (Audio|PlaySoundatLocation "/Game/Sound/boing.boing" HitLocation)
        (bind _output_get (Variables|Default|Setlastlocation HitLocation))))))

(fn ConstructionScript
  (|CallParentFunction))