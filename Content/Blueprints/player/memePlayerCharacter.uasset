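; Player character Blueprint for a first-person shooter, handling shooting, interaction, inventory, flashlight, health and death.
; Shooting line-traces from the FPS camera, spawns body-colored beam and spark particles, pushes physics objects, damages characters and launches the shooter.
; The use trace messages Interactable actors or picks up base items.
; Death ragdolls, switches to third-person, drops items and destroys the actor, while a Tick timer requests respawn through the game mode.
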(event Custom|suicide
  ;[1 1 1] DIE
  (Game|Damage|ApplyDamage self 5e+02 0 0 "/Game/Data/DT_Suicide.DT_Suicide_C"))

(event Custom|Request%20Spawn
  ;[1 1 1] RESPAWN
  (bind _asdefault_mode (Utilities|Casting|CastTodefaultMode (Game|GetGameMode)))
  (bind _asplayer_controller (Utilities|Casting|CastToPlayerController (Pawn|GetController)))
  (Default|Respawn _asdefault_mode _asplayer_controller))

(event Custom|Hitscan_Visuals
  (params (HitLocation :type Vector) (HitNormal :type Vector) (HitActor :type Actor%20Object%20Reference))
  (bind _returnvalue (Math|Conversions|RotationFromXVector HitNormal))
  (bind _returnvalue_2 (* HitNormal 5.0))
  (bind _mesh (Variables|Character|GetMesh))
  (bind _returnvalue_3 (Transformation|GetSocketLocation _mesh "laser"))
  (bind _returnvalue_4 (+ HitLocation _returnvalue_2))
  ;[1 1 1] Hitscan Visuals
  ;;[1 1 1] Create Laser Particles no matter what we hit
  (bind _returnvalue_5 (Effects|SpawnEmitterAttached "/Game/Particles/Beam/P_Beam.P_Beam" _mesh "laser" _returnvalue_3 (Variables|Default|Getrotation%20camera) "KeepWorldPosition"))
  ;;[1 1 1] Depending on the class, spawn or attach particles
  (bind _asserver_physicsobject (Utilities|Casting|CastToserver_physicsobject HitActor)
    (:then
      (bind _returnvalue_6 (Effects|SpawnEmitterAttached "/Game/Particles/P_Sparks.P_Sparks" (Variables|/Game/Blueprints/items/server_physicsobject.server_physicsobject_C|GetSM _asserver_physicsobject) "None" _returnvalue_4 _returnvalue "KeepWorldPosition"))
      (Physics|AddImpulseatLocation (Variables|/Game/Blueprints/items/server_physicsobject.server_physicsobject_C|GetSM _asserver_physicsobject) (* HitNormal -5e+03) HitLocation "None"))
    (:CastFailed
      (bind _returnvalue_7 (Effects|SpawnEmitteratLocation "/Game/Particles/P_Sparks.P_Sparks" _returnvalue_4 _returnvalue))))
  (Class|ParticleSystemComponent|SetBeamSourcePoint _returnvalue_5 0 _returnvalue_3)
  (Class|ParticleSystemComponent|SetBeamEndPoint _returnvalue_5 0 HitLocation)
  (Class|ParticleSystemComponent|SetBeamTargetPoint _returnvalue_5 0 HitLocation)
  (bind _returnvalue_8 (Rendering|Material|GetVectorParameterValue (Variables|Default|GetMaterial) "BodyColor" :!class /Script/Engine.MaterialInstanceDynamic))
  (Effects|Components|ParticleSystem|SetColorParameter _returnvalue_7 "colorStart" (Math|Color|MakeColor (.R (Math|Color|BreakColor _returnvalue_8)) (.G (Math|Color|BreakColor _returnvalue_8)) (.B (Math|Color|BreakColor _returnvalue_8))))
  (Effects|Components|ParticleSystem|SetColorParameter _returnvalue_7 "sparkColor" (Math|Color|MakeColor (.R (Math|Color|BreakColor _returnvalue_8)) (.G (Math|Color|BreakColor _returnvalue_8)) (.B (Math|Color|BreakColor _returnvalue_8))))
  (Audio|Components|Audio|Play (Variables|Default|Getflaunch) 0.0))

(event Custom|flash_light
  (params (state :type Boolean))
  ;[1 1 1] Flashlight
  (bind _output_get (Variables|Default|SetflashlightOn state))
  (CallFunction|FlashLightMulticast _output_get))

(event Custom|addToInventory
  (params (itemToAdd :type Base%20Object%20Reference))
  (bind _self self)
  (bind _inventory (Variables|Default|Getinventory))
  (bind _itemdata (Variables|/Game/Blueprints/items/item_data/base.base_C|GetitemData itemToAdd))
  (bind (_type _name _description _subtype) (Utilities|Struct|Breakitem_data _itemdata))
  ;[1 1 1] Inventory
  ;;[1 1 1] Adds an item inherited from base to the player's inventory.
  (if (not (Utilities|Array|ContainsItem _inventory itemToAdd))
    (Utilities|Array|AddUnique _inventory itemToAdd)
    (Default|OnPickedUp itemToAdd _self)
    (Development|PrintString (Utilities|String|ToString(Text) (Utilities|Text|FormatText "SRV {player} picked up a {subtype}! {item} was added to their inventory." (Utilities|Text|ToText(String) (Utilities|GetDisplayName (.ReturnValue (Class|VictoryBPFunctionLibrary|AccessorGetPlayerController _self)))) _subtype _name)) true true "(R=0.000000,G=1.000000,B=0.000000,A=1.000000)")))

(event Custom|request%20die
  ;[1 1 1] DIE
  (CallFunction|DIE))

(event Custom|Shoot
  (params (cameraRot :type Rotator))
  ;[1 1 1] Gun Hitscan
  (CallFunction|WeaponHitScan cameraRot))

(event Custom|Weapon%20HitScan
  (params (Camera%20Rot :type Rotator))
  (bind _self self)
  (bind _fps_cam (Variables|Default|Getfps_cam))
  (bind _returnvalue (Transformation|GetWorldLocation _fps_cam))
  ;[1 1 1] Gun Hitscan
  (Variables|Default|Setrotation%20camera Camera%20Rot)
  (bind (_outhit _returnvalue_2) (Collision|LineTraceByChannel _returnvalue (+ _returnvalue (* (Math|Vector|GetForwardVector (Variables|Default|Getrotation%20camera)) 5e+04)) "TraceTypeQuery1" false 0 "None"))
  (if _returnvalue_2
    (Variables|Default|Setlaser%20hit (.Location (Collision|BreakHitResult _outhit)))
    (else
      (Variables|Default|Setlaser%20hit (+ _returnvalue (* (Math|Vector|GetForwardVector (Variables|Default|Getrotation%20camera)) 5e+04)))))
  (CallFunction|HitscanVisuals (Variables|Default|Getlaser%20hit) (.ImpactNormal (Collision|BreakHitResult _outhit)) (.HitActor (Collision|BreakHitResult _outhit)))
  (bind _asmeme_player_character (Utilities|Casting|CastToMemePlayerCharacter (.HitActor (Collision|BreakHitResult _outhit)))
    (:then
      (Game|Damage|ApplyDamage _asmeme_player_character 5e+02 (.ReturnValue (Class|VictoryBPFunctionLibrary|AccessorGetPlayerController _self)) _self "/Game/Data/DT_Explosion.DT_Explosion_C"))
    (:CastFailed
      _))
  (Character|LaunchCharacter (* (Math|Vector|NegateVector (+ _returnvalue (* (Math|Vector|GetForwardVector (Variables|Default|Getrotation%20camera)) 5e+04))) "0.010000,0.010000,0.010000") false false))

(event Custom|Use%20Function
  (params (rot :type Rotator))
  (bind _fps_cam (Variables|Default|Getfps_cam))
  (bind _returnvalue (Transformation|GetWorldLocation _fps_cam))
  ;[1 1 1] Interact
  (bind _outhit (Collision|LineTraceByChannel _returnvalue (+ _returnvalue (* (Math|Vector|GetForwardVector rot) 1.5e+03)) "TraceTypeQuery1" false 0 "None"))
  (if (Utilities|DoesObjectImplementInterface (.HitActor (Collision|BreakHitResult _outhit)) "/Game/Blueprints/interface/Interactable.Interactable_C")
    (Class|Interactable|Interact(Message) (.HitActor (Collision|BreakHitResult _outhit)))
    (elif (Utilities|DoesObjectImplementInterface (.HitActor (Collision|BreakHitResult _outhit)) "/Game/Blueprints/items/item_data/base_interface.base_interface_C")
      (bind _asbase (Utilities|Casting|CastTobase (.HitActor (Collision|BreakHitResult _outhit))))
      (CallFunction|AddtoInventory _asbase))))

(event Custom|removeFromInventory
  (params (itemToRemove :type Base%20Object%20Reference))
  (bind _inventory (Variables|Default|Getinventory))
  (bind _itemdata (Variables|/Game/Blueprints/items/item_data/base.base_C|GetitemData itemToRemove))
  (bind (_type _name _description _subtype) (Utilities|Struct|Breakitem_data _itemdata))
  ;[1 1 1] Inventory
  ;;[1 1 1] Removes an item inherited from base from the player's inventory.
  (Utilities|Array|RemoveIndex _inventory (Utilities|Array|FindItem _inventory itemToRemove))
  (Default|OnDropped itemToRemove)
  (Development|PrintString (Utilities|String|ToString(Text) (Utilities|Text|FormatText "SRV {player} dropped a {subtype}! {item} was removed from their inventory." (Utilities|Text|ToText(String) (Utilities|GetDisplayName (.ReturnValue (Class|VictoryBPFunctionLibrary|AccessorGetPlayerController self)))) _subtype _name)) true true "(R=1.000000,G=1.000000,B=0.000000,A=1.000000)"))

(event Custom|flash_light_multicast
  (params (State :type Boolean))
  ;[1 1 1] Flashlight
  (Rendering|SetVisibility (Variables|Default|GetFlashlight) State false))

(event Custom|DropAllItems
  ;[1 1 1] Inventory
  ;;[1 1 1] Drop all items
  (for _array_element (Variables|Default|Getinventory)
    (CallFunction|RemovefromInventory _array_element)))

(event Custom|Enable%20FPS%20Camera
  ;[1 1 1] Camera Functions
  (Components|Activation|SetActive (Variables|Default|Getfps_cam) true false)
  (Components|Activation|SetActive (Variables|Default|GetFollowCamera) false false))

(event Custom|Enable%20TPS%20Camera
  ;[1 1 1] Camera Functions
  (Components|Activation|SetActive (Variables|Default|Getfps_cam) false false)
  (Components|Activation|SetActive (Variables|Default|GetFollowCamera) true false))

(event Custom|DIE
  (bind _self self)
  (bind _mesh (Variables|Character|GetMesh))
  (bind _returnvalue (Class|VictoryBPFunctionLibrary|AccessorGetPlayerController _self))
  ;[1 1 1] DIE
  (Variables|Default|Setdead true)
  (Physics|SetSimulatePhysics _mesh true)
  (Collision|SetCollisionProfileName _mesh "ragdoll" :!class /Script/Engine.PrimitiveComponent)
  (Input|DisableInput _returnvalue)
  (CallFunction|EnableTPSCamera)
  (CallFunction|DropAllItems)
  (bind _asmeme_player_controller (Utilities|Casting|CastToMemePlayerController _returnvalue)
    (:then
      (Default|UPDATEHUDonCLIENT _asmeme_player_controller self))
    (:CastFailed
      _))
  (Utilities|FlowControl|Delay 3.1)
  (Actor|DestroyActor self))

(event Custom|RESPAWN
  ;[1 1 1] RESPAWN
  (Variables|Default|Setdead false)
  (bind _asmeme_player_controller (Utilities|Casting|CastToMemePlayerController (Pawn|GetController)))
  (Utilities|IsValid (Pawn|GetControlledPawn _asmeme_player_controller)
    (:Is%20Valid
      (CallFunction|RequestSpawn)
      (Development|PrintString "WORKS"))))

(event Custom|Check%20Respawn
  (params (delta :type Float%20%28single-precision%29))
  ;[1 1 1] Check Respawn
  (if (Variables|Default|Getdead)
    (bind _output_get (Variables|Default|SetspawnTimer (+ delta (Variables|Default|GetspawnTimer))))
    (if (> _output_get 3.0)
      (CallFunction|RESPAWN)
      (Variables|Default|SetspawnTimer 0.0))))

(event Game|Damage|EventAnyDamage
  (params (Damage :type Float%20%28single-precision%29) (DamageType :type Damage%20Type%20Object%20Reference) (InstigatedBy :type Controller%20Object%20Reference) (DamageCauser :type Actor%20Object%20Reference))
  (bind _returnvalue (Utilities|GetDisplayName DamageCauser))
  (bind _returnvalue_2 (Utilities|GetDisplayName DamageType))
  (bind _self self)
  (bind _self_2 self)
  (bind _returnvalue_3 (Class|VictoryBPFunctionLibrary|AccessorGetPlayerController _self_2))
  (bind _returnvalue_4 (Class|VictoryBPFunctionLibrary|AccessorGetPlayerController _self))
  (bind _returnvalue_5 (Utilities|GetDisplayName _returnvalue_4))
  ;[1 1 1] Handle Damage
  (if (not (Variables|Default|Getdead))
    (if (> (- (Variables|Default|Gethealth) (Math|Float|Truncate Damage)) 0)
      (Variables|Default|Sethealth (- (Variables|Default|Gethealth) (Math|Float|Truncate Damage)))
      (bind _asmeme_player_controller (Utilities|Casting|CastToMemePlayerController _returnvalue_3))
      (Default|UPDATEHUDonCLIENT _asmeme_player_controller self)
      (else
        (Variables|Default|Sethealth 1)
        (Utilities|FlowControl|Delay 0.1)
        (bind _asmeme_player_controller_2 (Utilities|Casting|CastToMemePlayerController _returnvalue_3))
        (Default|UPDATEHUDonCLIENT _asmeme_player_controller_2 self)
        (CallFunction|RequestDie)
        (Utilities|Casting|CastToMemePlayerController InstigatedBy
          (:then
            (Development|PrintString (Utilities|String|Append "Player '" _returnvalue_5 "' was killed by '" (Utilities|GetDisplayName InstigatedBy) "' using weapon '" _returnvalue "' via '" _returnvalue_2 "'.") true true "(R=1.000000,G=0.000000,B=0.000000,A=1.000000)"))
          (:CastFailed
            (Development|PrintString (Utilities|String|Append "Player '" _returnvalue_5 "' was killed using '" _returnvalue "' via '" _returnvalue_2 "'.") true true "(R=1.000000,G=0.000000,B=0.000000,A=1.000000)")))))))

(event EventBeginPlay
  ;[1 1 1] Setup
  (Variables|Default|SetbUseControllerRotationYaw true)
  (CallFunction|EnableFPSCamera)
  (Variables|Default|SetmaxHealth 500)
  (Variables|Default|Sethealth 500))

(event EventTick
  (params (DeltaSeconds :type Float%20%28single-precision%29))
  ;[1 1 1] Could use a callback from gamemode here instead
  (CallFunction|CheckRespawn DeltaSeconds))

(event Input|KeyboardEvents|E
  (params (Key :type Key%20Structure :default "AnyKey"))
  ;[1 1 1] Interact
  (:Pressed
    (CallFunction|UseFunction (Transformation|GetWorldRotation (Variables|Default|Getfps_cam)))))

(event Input|KeyboardEvents|F
  (params (Key :type Key%20Structure :default "AnyKey"))
  ;[1 1 1] Flashlight
  (:Pressed
    (bind _isa (Utilities|FlowControl|FlipFlop)
      (:A
        _)
      (:B
        _))
    (bind _output_get (Variables|Default|SetflashlightOn _isa))
    (CallFunction|FlashLight _output_get)))

(event Input|KeyboardEvents|X
  (params (Key :type Key%20Structure :default "AnyKey"))
  ;[1 1 1] DIE
  (:Pressed
    (CallFunction|Suicide)))

(event Input|MouseEvents|LeftMouseButton
  (params (Key :type Key%20Structure :default "AnyKey"))
  ;[1 1 1] Gun Hitscan
  (:Pressed
    (if (not (Variables|Default|GetPaused)) ; Here I'll add a function that gets equipped weapon & fires it instead of calling shoot on the client.
      (CallFunction|Shoot (Transformation|GetWorldRotation (Variables|Default|Getfps_cam))))))

(fn ConstructionScript)